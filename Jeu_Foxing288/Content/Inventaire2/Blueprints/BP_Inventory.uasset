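; BP_Inventory is a slot-based inventory that stores an item class and amount per slot, in an array sized on BeginPlay.
; AddItem tops up partial stacks of stackable items before using empty slots, and gives non-stackable items one slot each.
; It recurses on any overflow and returns the amount that did not fit.
; Helper functions find free slots or stacks and report a slot's emptiness, class-default item info and amount.
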(event `self.ReceiveBeginPlay`
  (`KismetArrayLibrary.Array_Resize` (`self.Slots`) (`self.AmountOfSlots`)))

(fn `AddItem`
  (params (ItemClass :type "/Game/Inventaire2/Blueprints/ItemClasses/BP_MainItem Class Reference") (Amount :type Integer))
  (returns (`Success?` :type Boolean) (Rest :type Integer))
  (locals (localClass :type "/Game/Inventaire2/Blueprints/ItemClasses/BP_MainItem Class Reference") (`Local Amount` :type Integer) (FoundIndex :type Integer))
  (bind _returnvalue (+ (`.Amount_6_29DFF1764143514E51B820B573E53296` (break `/Game/Inventaire2/Blueprints/Structures/S_InventaireSlot` (`|GetArrayItem` (`self.Slots`) (`local.FoundIndex`)))) (`local.Local Amount`)))
  (set `local.localClass` ItemClass)
  (set `local.Local Amount` Amount)
  (if (`.CanbeStacked?_41_2D4B0F83439BB33F363BD49C5A14D333` (break `/Game/Inventaire2/Blueprints/Structures/S_ItemInfo` (defaults `/Game/Inventaire2/Blueprints/BP_Inventory` ItemClass)))
    (bind (_succes_ _index) (`self.SearchFreeStack` (`local.localClass`)))
    (if _succes_
      (set `local.FoundIndex` _index)
      (if (> _returnvalue (`self.Max Stack Size`))
        (set `local.Local Amount` (- _returnvalue (`self.Max Stack Size`)))
        (`KismetArrayLibrary.Array_Set` (`self.Slots`) (`local.FoundIndex`) (make `/Game/Inventaire2/Blueprints/Structures/S_InventaireSlot` (`local.localClass`) (`self.Max Stack Size`)))
        (bind (_success_ _rest) (`self.AddItem` (`local.localClass`) (`local.Local Amount`)))
        (return true _rest)
        (else
          (`KismetArrayLibrary.Array_Set` (`self.Slots`) (`local.FoundIndex`) (make `/Game/Inventaire2/Blueprints/Structures/S_InventaireSlot` (`local.localClass`) _returnvalue))
          (return true 0)))
      (else
        (bind (_succes__2 _index_2) (`self.SearchEmptySlot`))
        (if _succes__2
          (set `local.FoundIndex` _index_2)
          (if (> (`local.Local Amount`) (`self.Max Stack Size`))
            (`KismetArrayLibrary.Array_Set` (`self.Slots`) 0 (make `/Game/Inventaire2/Blueprints/Structures/S_InventaireSlot` (`local.localClass`) (`self.Max Stack Size`)))
            (bind (_success__2 _rest_2) (`self.AddItem` (`local.localClass`) (- (`local.Local Amount`) (`self.Max Stack Size`))))
            (return true _rest_2)
            (else
              (`KismetArrayLibrary.Array_Set` (`self.Slots`) (`local.FoundIndex`) (make `/Game/Inventaire2/Blueprints/Structures/S_InventaireSlot` (`local.localClass`) (`local.Local Amount`)))
              (return true 0)))
          (else
            (return false (`local.Local Amount`))))))
    (else
      (bind (_succes__3 _index_3) (`self.SearchEmptySlot`))
      (if _succes__3
        (bind _output_get (set `local.FoundIndex` _index_3))
        (`KismetArrayLibrary.Array_Set` (`self.Slots`) _output_get (make `/Game/Inventaire2/Blueprints/Structures/S_InventaireSlot` (`local.localClass`) 1))
        (if (> (`local.Local Amount`) 1)
          (bind (_success__3 _rest_3) (`self.AddItem` (`local.localClass`) (- (`local.Local Amount`) 1)))
          (return true _rest_3)
          (else
            (return true 0)))
        (else
          (return false (`local.Local Amount`)))))))

(fn `GetAmountIndex`
  (params (Index :type Integer))
  (returns (Amount :type Integer))
  (return (`.Amount_6_29DFF1764143514E51B820B573E53296` (break `/Game/Inventaire2/Blueprints/Structures/S_InventaireSlot` (`|GetArrayItem` (`self.Slots`) Index)))))

(fn `GetItemInfoAtIndex`
  (params (Index :type Integer))
  (returns (`EmptySlot?` :type Boolean) (ItemInfo :type "/Game/Inventaire2/Blueprints/Structures/S_ItemInfo Structure") (Amount :type Integer))
  (bind (_itemclass _amount) (break `/Game/Inventaire2/Blueprints/Structures/S_InventaireSlot` (`|GetArrayItem` (`self.Slots`) Index)))
  (if (`KismetSystemLibrary.IsValidClass` _itemclass)
    (return false (defaults `/Game/Inventaire2/Blueprints/BP_Inventory` _itemclass) _amount)
    (else
      (return true (struct) 0))))

(fn `IsSlotEmpty?`
  (params (Index :type Integer))
  (returns (`Empty ?` :type Boolean))
  (return (not (`KismetSystemLibrary.IsValidClass` (`.ItemClass_2_1C39CEF14ADD353EB869F5A7AD58259B` (break `/Game/Inventaire2/Blueprints/Structures/S_InventaireSlot` (`|GetArrayItem` (`self.Slots`) Index)))))))

(fn `SearchEmptySlot`
  (returns (`Succes?` :type Boolean) (Index :type Integer))
  (locals (LocalBool :type Boolean) (LocalIndex :type Integer))
  (for (_array_element _array_index) (`self.Slots`)
    (if (not (`KismetSystemLibrary.IsValidClass` (`.ItemClass_2_1C39CEF14ADD353EB869F5A7AD58259B` (break `/Game/Inventaire2/Blueprints/Structures/S_InventaireSlot` _array_element))))
      (set `local.LocalBool` true)
      (set `local.LocalIndex` _array_index)
      (break)))
  (return (`local.LocalBool`) (`local.LocalIndex`)))

(fn `SearchFreeStack`
  (params (ItemClass :type "/Game/Inventaire2/Blueprints/ItemClasses/BP_MainItem Class Reference"))
  (returns (`Succes?` :type Boolean) (Index :type Integer))
  (locals (LocalBool :type Boolean) (LocalIndex :type Integer))
  (for (_array_element _array_index) (`self.Slots`)
    (bind (_itemclass _amount) (break `/Game/Inventaire2/Blueprints/Structures/S_InventaireSlot` _array_element))
    (if (`KismetSystemLibrary.IsValidClass` _itemclass)
      (if (and (== _itemclass ItemClass) (< _amount (`self.Max Stack Size`)))
        (set `local.LocalBool` true)
        (set `local.LocalIndex` _array_index)
        (break))))
  (return (`local.LocalBool`) (`local.LocalIndex`)))

(fn `UserConstructionScript`)